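; Tunnel segment actor for an endless-runner style level, with a rotating holed wall, a healthpack and an enemy, the latter two randomly offset on BeginPlay.
; Passing the trigger zone has TunnelSpawner spawn a tunnel, destroys this one and adds score.
; Overlaps update BP_Player health and score directly, with camera shake on damage and projectiles killing the enemy.
; RandomizeWall and RandomizeHealthPack vary wall mesh, roll and healthpack presence, but are not called here.
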(event OnComponentBeginOverlap(TriggerZone)
  (params (OverlappedComponent :type Primitive%20Component%20Object%20Reference) (OtherActor :type Actor%20Object%20Reference) (OtherComp :type Primitive%20Component%20Object%20Reference) (OtherBodyIndex :type Integer) (bFromSweep :type Boolean) (SweepResult :type Hit%20Result%20Structure%20%28by%20ref%29))
  (bind _asbp_player (Utilities|Casting|CastToBP_Player OtherActor))
  (Utilities|FlowControl|Sequence
    (:then_0
      (Default|SpawnTunnelatSpawnPoint (Variables|Default|GetTunnelSpawner))
      (Actor|DestroyActor))
    (:then_1
      (bind _output_get (Variables|/Game/InfiniteMatrix/Blueprints/BP_Player.BP_Player_C|SettmpScore _asbp_player (+ (Variables|/Game/InfiniteMatrix/Blueprints/BP_Player.BP_Player_C|GettmpScore _asbp_player) 1)))
      (Variables|/Game/InfiniteMatrix/Blueprints/BP_Player.BP_Player_C|SetScore _asbp_player _output_get))))

(event OnComponentBeginOverlap(WallMesh)
  (params (OverlappedComponent :type Primitive%20Component%20Object%20Reference) (OtherActor :type Actor%20Object%20Reference) (OtherComp :type Primitive%20Component%20Object%20Reference) (OtherBodyIndex :type Integer) (bFromSweep :type Boolean) (SweepResult :type Hit%20Result%20Structure%20%28by%20ref%29))
  (bind _asbp_player (Utilities|Casting|CastToBP_Player OtherActor))
  (Utilities|FlowControl|Sequence
    (:then_0
      (bind _output_get (Variables|/Game/InfiniteMatrix/Blueprints/BP_Player.BP_Player_C|SetHealth _asbp_player (- (Variables|/Game/InfiniteMatrix/Blueprints/BP_Player.BP_Player_C|GetHealth _asbp_player) 1.0)))
      (if (<= _output_get 0.0)
        (Variables|/Game/InfiniteMatrix/Blueprints/BP_Player.BP_Player_C|SetIsDead _asbp_player true)
        (Default|DisplayRestart _asbp_player)
        (else
          (Camera|PlayWorldCameraShake "/Game/InfiniteMatrix/Blueprints/CameraShake.CameraShake_C" (Transformation|GetActorLocation _asbp_player) 0.0 5e+02))))
    (:then_1
      (Variables|/Game/InfiniteMatrix/Blueprints/BP_Player.BP_Player_C|SettmpScore _asbp_player (- (Variables|/Game/InfiniteMatrix/Blueprints/BP_Player.BP_Player_C|GettmpScore _asbp_player) 1)))))

(event OnComponentBeginOverlap(Healthpack)
  (params (OverlappedComponent :type Primitive%20Component%20Object%20Reference) (OtherActor :type Actor%20Object%20Reference) (OtherComp :type Primitive%20Component%20Object%20Reference) (OtherBodyIndex :type Integer) (bFromSweep :type Boolean) (SweepResult :type Hit%20Result%20Structure%20%28by%20ref%29))
  (bind _asbp_player (Utilities|Casting|CastToBP_Player OtherActor))
  (if (not (> (+ (Variables|/Game/InfiniteMatrix/Blueprints/BP_Player.BP_Player_C|GetHealth _asbp_player) 1.0) 1e+01))
    (Variables|/Game/InfiniteMatrix/Blueprints/BP_Player.BP_Player_C|SetHealth _asbp_player (+ (Variables|/Game/InfiniteMatrix/Blueprints/BP_Player.BP_Player_C|GetHealth _asbp_player) 1.0))
    (Components|DestroyComponent (Variables|Default|GetHealthpack))))

(event OnComponentBeginOverlap(Enemy)
  (params (OverlappedComponent :type Primitive%20Component%20Object%20Reference) (OtherActor :type Actor%20Object%20Reference) (OtherComp :type Primitive%20Component%20Object%20Reference) (OtherBodyIndex :type Integer) (bFromSweep :type Boolean) (SweepResult :type Hit%20Result%20Structure%20%28by%20ref%29))
  (Utilities|FlowControl|Sequence
    (:then_0
      (bind _asbp_projectile (Utilities|Casting|CastToBP_Projectile OtherActor))
      (Variables|/Game/InfiniteMatrix/Blueprints/BP_Player.BP_Player_C|SetScore (Variables|/Game/InfiniteMatrix/Blueprints/BP_Projectile.BP_Projectile_C|GetOwningPlayer _asbp_projectile) (+ (Variables|/Game/InfiniteMatrix/Blueprints/BP_Player.BP_Player_C|GetScore (Variables|/Game/InfiniteMatrix/Blueprints/BP_Projectile.BP_Projectile_C|GetOwningPlayer _asbp_projectile)) 1))
      (Components|DestroyComponent (Variables|Default|GetEnemy)))
    (:then_1
      (bind _asbp_player (Utilities|Casting|CastToBP_Player OtherActor))
      (Variables|/Game/InfiniteMatrix/Blueprints/BP_Player.BP_Player_C|SetHealth _asbp_player (- (Variables|/Game/InfiniteMatrix/Blueprints/BP_Player.BP_Player_C|GetHealth _asbp_player) 1.0))
      (Components|DestroyComponent (Variables|Default|GetEnemy))
      (Camera|PlayWorldCameraShake "/Game/InfiniteMatrix/Blueprints/CameraShake.CameraShake_C" (Transformation|GetActorLocation _asbp_player) 0.0 5e+02))))

(event EventBeginPlay
  (bind _randomloactionoffsetvec (CallFunction|RandomLocationOffset))
  (Transformation|AddLocalOffset (Variables|Default|GetHealthpack) _randomloactionoffsetvec false false)
  (bind _randomloactionoffsetvec_2 (CallFunction|RandomLocationOffset))
  (Transformation|AddLocalOffset (Variables|Default|GetEnemy) _randomloactionoffsetvec_2 false false))

(event EventTick
  (params (DeltaSeconds :type Float%20%28single-precision%29))
  (Transformation|AddLocalRotation (Variables|Default|GetWallMesh) (Math|Rotator|MakeRotator (* DeltaSeconds (Variables|Default|GetRotateSpeed)) 0.0 0.0) false false))

(fn ConstructionScript)

(fn RandomizeWall
  (Components|StaticMesh|SetStaticMesh (Variables|Default|GetWallMesh) (Utilities|Select :Index (Math|Random|RandomIntegerinRange 0 3) :Option%200 "/Game/InfiniteMatrix/Meshes/SM_Hole_01.SM_Hole_01" :Option%201 "/Game/InfiniteMatrix/Meshes/SM_Hole_02.SM_Hole_02" :Option%202 "/Game/InfiniteMatrix/Meshes/SM_Hole_03.SM_Hole_03" :Option%203 "/Game/InfiniteMatrix/Meshes/SM_Hole_04.SM_Hole_04"))
  (Transformation|AddLocalRotation (Variables|Default|GetWallMesh) (Math|Rotator|MakeRotator (Math|Random|RandomFloatinRange 0.0 3.6e+02) 0.0 0.0) false false))

(fn RandomizeHealthPack
  (params (isVisibile :type Boolean))
  (bind _healthpack (Variables|Default|GetHealthpack))
  (if isVisibile
    (Rendering|SetVisibility _healthpack true false)
    (Collision|SetCollisionEnabled _healthpack "QueryAndPhysics")
    (else
      (Rendering|SetVisibility _healthpack false false)
      (Collision|SetCollisionEnabled _healthpack "NoCollision"))))

(fn RandomLocationOffset
  (return (Math|Conversions|ToVector(Float) (Utilities|Struct|MakeIntVector (Math|Random|RandomIntegerinRange -100 100) (Math|Random|RandomIntegerinRange -200 200) (Math|Random|RandomIntegerinRange -200 200)))))